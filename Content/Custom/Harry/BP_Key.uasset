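; BP_Key is a key pickup that the player collects by pressing E while standing near it.
; Begin and end overlap events with BP_Player toggle an InRange flag and store the player reference.
; Tick polls the E key directly on player controller 0, then sets the stored player's HasKey to true and destroys the key actor.
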(event `self.ReceiveActorEndOverlap`
  (params (OtherActor :type "Actor Object Reference"))
  (cast `/Game/Blueprints/BP_Player` OtherActor)
  (set `self.In Range` false))

(event `self.ReceiveActorBeginOverlap`
  (params (OtherActor :type "Actor Object Reference"))
  (bind _asbp_player (cast `/Game/Blueprints/BP_Player` OtherActor))
  (set `self.In Range` true))

(event `self.ReceiveTick`
  (params (DeltaSeconds :type "Float (single-precision)"))
  (if (and (`PlayerController.IsInputKeyDown` (`GameplayStatics.GetPlayerController` 0) "E") (`self.In Range`))
    (set `/Game/Blueprints/BP_Player.HasKey` true (stale `self.ReceiveActorBeginOverlap` _asbp_player))
    (`self.K2_DestroyActor`)))

(fn `UserConstructionScript`)