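; BP_Bell is a trigger actor that rings a bell and then ends the game.
; When the player pawn begins overlapping its Box, it plays the Audio component three times, spaced by Delay nodes.
; After a final, longer delay it quits the game.
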(event `self.Box.OnComponentBeginOverlap`
  (params (OverlappedComponent :type "PrimitiveComponent Object Reference") (OtherActor :type "Actor Object Reference") (OtherComp :type "PrimitiveComponent Object Reference") (OtherBodyIndex :type Integer) (bFromSweep :type Boolean) (SweepResult :type "HitResult Structure (by ref)"))
  (if (== OtherActor (`GameplayStatics.GetPlayerPawn` 0))
    (`AudioComponent.Play` (`self.Audio`) 0.0)
    (`KismetSystemLibrary.Delay` 3.5)
    (`AudioComponent.Play` (`self.Audio`) 0.0)
    (`KismetSystemLibrary.Delay` 3.5)
    (`AudioComponent.Play` (`self.Audio`) 0.0)
    (`KismetSystemLibrary.Delay` 7.0)
    (`KismetSystemLibrary.QuitGame` null "Quit")))

(fn `UserConstructionScript`)